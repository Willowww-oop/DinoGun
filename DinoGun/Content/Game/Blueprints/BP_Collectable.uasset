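; BP_Collectable is a spinning pickup actor that the zombie character collects as a coin.
; On overlap with BP_ZombieCharacter it calls CollectCoin on the character, plays explosion and cheering sounds at its location, then destroys itself.
; Tick yaws the SMMaurice component by RotationPerSecond scaled by delta time for a frame-rate independent spin.
; An unconnected SpawnActor node never runs.
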(event EventBeginPlay)

(event Collision|EventActorBeginOverlap
  (params (OtherActor :type Actor%20Object%20Reference))
  (bind _returnvalue (Transformation|GetActorLocation))
  ;[0.15 0.15 0.15 0.5] Collision
  (bind _asbp_zombie_character (Utilities|Casting|CastToBP_ZombieCharacter OtherActor))
  (Default|CollectCoin _asbp_zombie_character)
  (Audio|PlaySoundatLocation "/Game/Game/Audio/A_Explosion.A_Explosion" _returnvalue "0, 0, 0" 1.0 1.0 0.0 0 0 0 0)
  (Audio|PlaySoundatLocation "/Game/Game/Audio/A_Cheering.A_Cheering" _returnvalue "0, 0, 0" 1.0 1.0 0.0 0 0 0 0)
  (Actor|DestroyActor))

(event EventTick
  (params (DeltaSeconds :type Float%20%28single-precision%29))
  ;[0.15 0.15 0.15 0.5] Rotation
  (Transformation|AddLocalRotation (Variables|Default|GetSM_Maurice) (Math|Rotator|MakeRotator 0.0 0.0 (* DeltaSeconds (Variables|Default|GetRotationPerSecond))) false false))

(fn ConstructionScript)