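; BP_Damageable is an actor that takes damage, tracks health and awards points when destroyed.
; Its construction script applies a configurable Mesh to its static mesh component.
; AnyDamage subtracts damage from Health; at zero or below, it passes PointWorth to AddPoints on BP_PawnGameInstance and destroys itself, provided that game instance cast succeeds.
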(event EventBeginPlay)

(event Collision|EventActorBeginOverlap
  (params (OtherActor :type Actor%20Object%20Reference)))

(event EventTick
  (params (DeltaSeconds :type Float%20%28single-precision%29)))

(event Game|Damage|EventAnyDamage
  (params (Damage :type Float%20%28single-precision%29) (DamageType :type Damage%20Type%20Object%20Reference) (InstigatedBy :type Controller%20Object%20Reference) (DamageCauser :type Actor%20Object%20Reference))
  (Variables|Default|SetHealth (- (Variables|Default|GetHealth) Damage))
  (if (<= (Variables|Default|GetHealth) 0.0)
    (bind _asbp_pawn_game_instance (Utilities|Casting|CastToBP_PawnGameInstance (Game|GetGameInstance)))
    (Default|AddPoints _asbp_pawn_game_instance (Variables|Default|GetPointWorth))
    (Actor|DestroyActor)))

(fn ConstructionScript
  (Components|StaticMesh|SetStaticMesh (Variables|Default|GetStaticMesh) (Variables|Default|GetMesh)))