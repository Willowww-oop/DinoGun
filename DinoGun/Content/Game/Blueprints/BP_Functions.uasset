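; BP_Functions is a Blueprint collection of small utility functions for toggling actors and measuring angles.
; EnableActor and DisableActor switch an actor's visibility, collision and tick together, acting as a reversible alternative to spawning or destroying.
; SignedAngle takes the arccosine of two vectors' dot product and negates it when their cross product's Z is negative, without normalizing the inputs.
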(fn EnableActor
  (params (Actor :type Actor%20Object%20Reference))
  (Rendering|SetActorHiddenInGame Actor false)
  (Collision|SetActorEnableCollision Actor true)
  (Actor|Tick|SetActorTickEnabled Actor true))

(fn DisableActor
  (params (Actor :type Actor%20Object%20Reference))
  (Rendering|SetActorHiddenInGame Actor true)
  (Collision|SetActorEnableCollision Actor false)
  (Actor|Tick|SetActorTickEnabled Actor))

(fn SignedAngle
  (params (A :type Vector) (B :type Vector))
  (bind _returnvalue (Math|Vector|DotProduct A B))
  (bind _returnvalue_2 (Math|Trig|Acos(Degrees) _returnvalue))
  (if (< (.z (Math|Vector|CrossProduct A B)) 0.0)
    (return (* _returnvalue_2 -1.0))
    (else
      (return _returnvalue_2))))