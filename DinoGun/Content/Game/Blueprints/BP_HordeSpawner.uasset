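; Wave spawner that sends growing hordes of random enemy types around a BP_ZombieCharacter stored as the player.
; On BeginPlay it picks that character from the level, then starts the first wave after a short delay.
; Each wave spawns enemies at random navmesh points near the character, passing itself as HordeManager, then scales up the next count.
; EnemyDied decrements the live count and launches the next wave, after a delay, once none remain.
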(event Custom|EnemyDied
  (bind _enemycount (Variables|Default|GetEnemyCount))
  (Math|Integer|DecrementInt _enemycount
    (:%20%20
      (if (<= _enemycount 0)
        (Utilities|FlowControl|Delay 5.0)
        (CallFunction|SpawnHorde)))))

(event Custom|SpawnHorde
  (for _index (range 1 (Variables|Default|GetStartingHordeCount))
    (bind _randomlocation (Class|NavigationSystemV1|GetRandomLocationinNavigableRadius (Transformation|GetActorLocation (Variables|Default|GetPlayerCharacter)) 1e+03 0 0))
    (Game|SpawnActorfromClass (.OutItem (Utilities|Array|Random (Variables|Default|GetEnemyTypes))) (Math|Transform|MakeTransform _randomlocation "0, 0, 0" "1.000000,1.000000,1.000000") "AdjustIfPossibleButAlwaysSpawn" "MultiplyWithRoot" 0 self 0)
    (Math|Integer|IncrementInt (Variables|Default|GetEnemyCount)))
  (Variables|Default|SetStartingHordeCount (* (Variables|Default|GetStartingHordeCount) 1.5))
  (Math|Integer|IncrementInt (Variables|Default|GetWaveNumber)))

(event EventBeginPlay
  (bind _outactors (Actor|GetAllActorsOfClass "/Game/Game/Characters/Zombie/Blueprints/BP_ZombieCharacter.BP_ZombieCharacter_C"))
  (Variables|Default|SetPlayerCharacter (.OutItem (Utilities|Array|Random _outactors)))
  (Utilities|FlowControl|Delay 5.0)
  (CallFunction|SpawnHorde))

(fn ConstructionScript)