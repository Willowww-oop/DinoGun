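; BP_PawnGameInstance is a game instance that tracks the player's lives and score for the session.
; StartGame resets both to their starting values, and AddPoints adds to the score and prints the total.
; LoseLife decrements lives and only prints a debug message when they run out, with no game-over logic.
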(fn StartGame
  (Variables|Default|SetLives 3)
  (Variables|Default|SetScore 0))

(fn AddPoints
  (params (Points :type Integer))
  (Variables|Default|SetScore (+ Points (Variables|Default|GetScore)))
  (Development|PrintString (Utilities|String|ToString(Integer) (Variables|Default|GetScore))))

(fn LoseLife
  (bind _lives (Variables|Default|GetLives))
  (Math|Integer|DecrementInt _lives
    (:%20%20
      (if (<= _lives 0)
        (Development|PrintString "Imagine dying lmao")))))