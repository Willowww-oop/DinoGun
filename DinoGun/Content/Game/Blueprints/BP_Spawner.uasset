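; Spawner actor that creates one instance of a configurable actor class at its own location, raised by a height modifier.
; DoSpawn, which nothing in this file calls, spawns only while CanSpawn is true, then clears the flag.
; The flag starts true on BeginPlay and is restored when an actor of the spawned class ends overlap with the spawner, gating repeat spawns.
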(event EventBeginPlay
  (Variables|Default|SetCanSpawn true))

(event EventTick
  (params (DeltaSeconds :type Float%20%28single-precision%29)))

(event Collision|EventActorEndOverlap
  (params (OtherActor :type Actor%20Object%20Reference))
  (Class|KismetSystemLibrary|IsObjectOfSoftClass OtherActor (Utilities|ResolveSoftReference (Variables|Default|GetSpawnActor))
    (:True
      (Variables|Default|SetCanSpawn true))))

(fn ConstructionScript)

(fn DoSpawn
  (bind _returnvalue (Transformation|GetActorLocation))
  (if (Variables|Default|GetCanSpawn)
    (Game|SpawnActorfromClass (Variables|Default|GetSpawnActor) (Math|Transform|MakeTransform (Math|Vector|MakeVector (.x _returnvalue) (.y _returnvalue) (+ (.z _returnvalue) (Variables|Default|GetHeightModifier))) "0, 0, 0" "1.000000,1.000000,1.000000") "Undefined" "MultiplyWithRoot" 0 0)
    (Variables|Default|SetCanSpawn false)))