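; AI controller for armed enemies that runs the enemy behavior tree and fires a weapon on perceiving the player.
; On possession it stores a random BP_ZombieCharacter as the blackboard's EnemyActor.
; Sensing a Player-tagged actor cancels the timer, sets HasLineOfSight and starts firing; other perception updates start a delay that clears the flag and stops fire.
; Death stops fire and disables perception responses.
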(event OnTargetPerceptionUpdated(AIPerception)
  (params (Actor :type Actor%20Object%20Reference) (Stimulus :type AI%20Stimulus%20Structure))
  (if (not (Variables|Default|GetDead))
    (if (and (Actor|ActorHasTag Actor "Player") (.bSuccessfullySensed (Utilities|Struct|BreakAIStimulus Stimulus)))
      (Utilities|Time|ClearandInvalidateTimerbyHandle (Variables|Default|GetEnemyTimer))
      (AI|Components|Blackboard|SetValueasBool (Variables|Default|GetBlackboard) (Variables|Default|GetHas%20Line%20of%20Sight) true)
      (Default|OnStartFire (Variables|Default|GetWeapon))
      (else
        (bind _returnvalue (Utilities|Time|SetTimerbyEvent (delegate Custom|StartEnemyTimer) (Variables|Default|GetLine%20of%20Sight%20Timer)))
        (Variables|Default|SetEnemyTimer _returnvalue)))))

(event Custom|StartEnemyTimer
  (AI|Components|Blackboard|SetValueasBool (Variables|Default|GetBlackboard) (Variables|Default|GetHas%20Line%20of%20Sight) false)
  (Default|OnStopFire (Variables|Default|GetWeapon)))

(event Custom|Die
  (Variables|Default|SetDead true)
  (Default|OnStopFire (Variables|Default|GetWeapon)))

(event EventBeginPlay)

(event EventTick
  (params (DeltaSeconds :type Float%20%28single-precision%29)))

(event EventPossess
  (params (PossessedPawn :type Pawn%20Object%20Reference))
  (AI|RunBehaviorTree "/Game/Game/Characters/Enemy/Blueprints/BT_Enemy.BT_Enemy")
  (bind _outactors (Actor|GetAllActorsOfClass "/Game/Game/Characters/Zombie/Blueprints/BP_ZombieCharacter.BP_ZombieCharacter_C"))
  (AI|Components|Blackboard|SetValueasObject (Variables|Default|GetBlackboard) (Variables|Default|GetEnemyActor) (.OutItem (Utilities|Array|Random _outactors))))

(fn ConstructionScript)