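; BP_AOE is a short-lived area-of-effect damage actor for weapons.
; It applies its Damage value to any actor that begins overlapping it, skipping its owner.
; It destroys itself after a brief fixed delay from BeginPlay; its Lifespan variable is unused.
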(event EventBeginPlay
  (|CallParentFunction)
  (Utilities|FlowControl|Delay 0.2)
  (Actor|DestroyActor))

(event Collision|EventActorBeginOverlap
  (params (OtherActor :type Actor%20Object%20Reference))
  (|CallParentFunction OtherActor)
  (if (!= OtherActor (Components|GetOwner))
    (Game|Damage|ApplyDamage OtherActor (Variables|Default|GetDamage) 0 0)))

(event EventTick
  (params (DeltaSeconds :type Float%20%28single-precision%29))
  (|CallParentFunction DeltaSeconds) ; This node is disabled and will not be called.\nDrag off pins to build functionality.
)

(fn ConstructionScript
  (|CallParentFunction))