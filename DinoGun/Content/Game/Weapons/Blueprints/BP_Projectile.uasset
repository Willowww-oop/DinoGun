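; Projectile actor for weapons that damages what it overlaps and then destroys itself.
; The construction script applies Speed to the ProjectileMovement component's initial speed and sets the actor's lifespan from Lifespan.
; On overlap it calls the parent handler, then ignores actors carrying SourceTag; any other actor receives Damage before the projectile is destroyed.
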(event EventBeginPlay
  (|CallParentFunction) ; This node is disabled and will not be called.\nDrag off pins to build functionality.
)

(event Collision|EventActorBeginOverlap
  (params (OtherActor :type Actor%20Object%20Reference))
  (|CallParentFunction OtherActor)
  (if (not (Actor|ActorHasTag OtherActor (Variables|Default|GetSourceTag)))
    (Game|Damage|ApplyDamage OtherActor (Variables|Default|GetDamage) 0 0)
    (Actor|DestroyActor)))

(event EventTick
  (params (DeltaSeconds :type Float%20%28single-precision%29))
  (|CallParentFunction DeltaSeconds) ; This node is disabled and will not be called.\nDrag off pins to build functionality.
)

(fn ConstructionScript
  (|CallParentFunction)
  (Variables|/Script/Engine.ProjectileMovementComponent|SetInitialSpeed (Variables|Default|GetProjectileMovement) (Variables|Default|GetSpeed))
  (Actor|SetLifeSpan (Variables|Default|GetLifespan)))